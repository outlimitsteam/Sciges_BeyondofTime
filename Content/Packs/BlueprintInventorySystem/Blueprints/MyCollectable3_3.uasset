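; Collectable pickup actor from a Blueprint inventory system that adds one to a Collectable3 count when its mesh is overlapped.
; Any overlap destroys the mesh component, leaving the actor in place, then increments the counter after casting the first actor from a class search.
; A pickup sound plays only if the overlapping actor passes a second cast, at half pitch while SlowMotion is active.
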(event OnComponentBeginOverlap(StaticMesh1)
  (params (OtherActor :type Actor%20Object%20Reference) (OtherComp :type Primitive%20Component%20Object%20Reference) (OtherBodyIndex :type Integer) (bFromSweep :type Boolean) (SweepResult :type Hit%20Result%20Structure%20%28by%20ref%29))
  (bind _returnvalue (Transformation|GetActorLocation))
  (Components|DestroyComponent (Variables|Default|GetStaticMesh1))
  (bind _outactors (Actor|GetAllActorsOfClass 0))
  (Utilities|Casting|CastTo (Utilities|Array|Get(acopy) _outactors))
  (Variables|Default|SetCollectable%203 (+ (Variables|Default|GetCollectable%203) 1))
  (Utilities|Casting|CastTo OtherActor)
  (if (Variables|Default|GetSlow%20Motion)
    (Audio|PlaySoundatLocation 0 _returnvalue 1.0 0.5)
    (else
      (Audio|PlaySoundatLocation 0 _returnvalue 1.0 1.0))))

(fn ConstructionScript)