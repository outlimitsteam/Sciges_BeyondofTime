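; Ammo type 5 pickup that grants extra ammo when an actor overlaps its box.
; The overlap destroys the pickup before the cast check, then sets the extra-ammo variable and plays a sound, pitched lower during slow motion.
; Each tick, the whole actor rotates along the line from the player camera to its text render, a look-at-player effect.
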(event OnComponentBeginOverlap(Box1)
  (params (OtherActor :type Actor%20Object%20Reference) (OtherComp :type Primitive%20Component%20Object%20Reference) (OtherBodyIndex :type Integer) (bFromSweep :type Boolean) (SweepResult :type Hit%20Result%20Structure%20%28by%20ref%29))
  (bind _returnvalue (Transformation|GetActorLocation))
  (Actor|DestroyActor)
  (Components|DestroyComponent (Variables|Default|GetBox1))
  (Utilities|Casting|CastTo OtherActor)
  (Variables|Default|SetAmmo%205%20-%20Extra%20[from%20"AmmoPickup5"%20BP] 30)
  (if (Variables|Default|GetSlow%20Motion)
    (Audio|PlaySoundatLocation 0 _returnvalue 1.0 0.8)
    (else
      (Audio|PlaySoundatLocation 0 _returnvalue 1.0 1.5))))

(event EventTick
  (params (DeltaSeconds :type Float%20%28single-precision%29))
  ;[1 1 1] Look/Face At Player
  (Transformation|SetActorRotation (Math|Rotator|FindLookatRotation (Transformation|GetActorLocation (Game|GetPlayerCameraManager 0)) (Transformation|GetWorldLocation (Variables|Default|GetTextRender1)))))

(fn ConstructionScript)