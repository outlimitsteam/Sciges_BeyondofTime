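; MyWeapon11 is a pickup weapon actor that the player collects by pressing E nearby.
; Box1 overlap shows a text prompt and enables input, both reverted on exit.
; Pickup destroys box and text, casts the overlapping actor to set IveWeapon11, then hides the weapon, disables physics and attaches it to the character's Weapon socket.
; A pickup sound plays with lower pitch during slow motion.
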(event OnComponentEndOverlap(Box1)
  (params (OtherActor :type Actor%20Object%20Reference) (OtherComp :type Primitive%20Component%20Object%20Reference) (OtherBodyIndex :type Integer))
  ;[1 1 1] Text Render Visibility
  (Input|DisableInput (Game|GetPlayerController 0))
  (Rendering|SetVisibility (Variables|Default|GetTextRender1) false false))

(event OnComponentBeginOverlap(Box1)
  (params (OtherActor :type Actor%20Object%20Reference) (OtherComp :type Primitive%20Component%20Object%20Reference) (OtherBodyIndex :type Integer) (bFromSweep :type Boolean) (SweepResult :type Hit%20Result%20Structure%20%28by%20ref%29))
  ;[1 1 1] Text Render Visibility
  (Input|EnableInput (Game|GetPlayerController 0))
  (Rendering|SetVisibility (Variables|Default|GetTextRender1) true false))

(event EventBeginPlay
  ;[1 1 1] Text Render Visibility
  (Rendering|SetVisibility (Variables|Default|GetTextRender1) false false))

(event Input|KeyboardEvents|E
  (bind _returnvalue (Transformation|GetActorLocation))
  ;[1 1 1] Pickup Weapon
  (:Pressed
    (Input|DisableInput 0)
    (Components|DestroyComponent (Variables|Default|GetBox1))
    (Utilities|Casting|CastTo (stale OnComponentBeginOverlap(Box1) OtherActor))
    (Variables|Default|SetI've%20Weapon%2011 true)
    (Rendering|SetActorHiddenInGame true)
    (Physics|SetSimulatePhysics (Variables|Default|GetStaticMesh1) false)
    (Class|Actor|AttachRootComponentto (Variables|/Script/Engine.Character|GetMesh (Game|GetPlayerCharacter 0)) "Weapon" "SnapToTarget" true)
    (if (Variables|Default|GetSlow%20Motion)
      (Audio|PlaySoundatLocation 0 _returnvalue 1.0 0.8)
      (else
        (Audio|PlaySoundatLocation 0 _returnvalue 1.0 1.5)))))

(fn ConstructionScript)