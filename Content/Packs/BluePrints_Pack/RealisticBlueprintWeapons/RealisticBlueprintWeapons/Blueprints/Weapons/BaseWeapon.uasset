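; Base weapon Blueprint with single shot, burst and full auto fire modes, cycling through those the weapon enables.
; SRV_Fire runs burst and full auto as Retriggerable Delay loops in the EventGraph, since functions cannot hold delays, while Tick accumulates cooldown timers.
; Authority-gated Fire checks ammo, rolls a random jam, then spawns a projectile at the Muzzle socket, passing it the weapon's ballistics and damage values.
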(event Custom|SRV_Fire
  (switch Utilities|FlowControl|Switch|Switchon (Variables|CurrentState|GetCurrentFireMode)
    (:NewEnumerator0
      ;[1 1 1] Single shot
      (Utilities|IsValid self
        (:Is%20Valid
          (FiringMechanics|Fire))))
    (:NewEnumerator1
      ;[1 1 1] No delay inside functions in UE4, loop placed here
      (if (> (Variables|CurrentState|GetTimeSinceLastBurst) (Variables|Stats|GetBurstDelay))
        (Variables|CurrentState|SetTimeSinceLastBurst 0.0)
        (if (> (Variables|Stats|GetBurstCount) (Variables|CurrentState|GetCurrentShotInBurst)) :!label _label
          (FiringMechanics|Fire)
          (Utilities|FlowControl|RetriggerableDelay (Variables|Stats|GetFireRateBurst))
          (goto _label)
          (else
            (Variables|CurrentState|SetCurrentShotInBurst 0)))))
    (:NewEnumerator2
      ;[1 1 1] No delay inside functions in UE4, loop placed here
      (if (Variables|CurrentState|GetTriggerPulled) :!label _label_2
        (FiringMechanics|Fire)
        (Utilities|FlowControl|RetriggerableDelay (Variables|Stats|GetFireRateFullAuto))
        (goto _label_2)))))

(event EventTick
  (params (DeltaSeconds :type Float%20%28single-precision%29))
  ;[1 1 1] Setting timers for single shot or burst shot.
  (Variables|CurrentState|SetTimeSinceLastShot (+ DeltaSeconds (Variables|CurrentState|GetTimeSinceLastShot)))
  (Variables|CurrentState|SetTimeSinceLastBurst (+ DeltaSeconds (Variables|CurrentState|GetTimeSinceLastBurst))))

(fn ConstructionScript
  (Physics|SetSimulatePhysics (Variables|Cosmetics|GetWeaponMesh) true))

(fn Fire
  (Networking|SwitchHasAuthority
    (:Authority
      (bind _hasammo (Checks|HasAmmo))
      (if _hasammo
        (switch Utilities|FlowControl|Switch|Switchon (Variables|CurrentState|GetCurrentFireMode)
          (:NewEnumerator0
            (FiringMechanics|FireSingle))
          (:NewEnumerator1
            (FiringMechanics|FireBurst))
          (:NewEnumerator2
            (FiringMechanics|FireFullAuto)))
        (else
          (FiringMechanics|TriggerNoAmmo))))))

(fn FireSingle
  (Networking|SwitchHasAuthority
    (:Authority
      (if (>= (Variables|CurrentState|GetTimeSinceLastShot) (Variables|Stats|GetFireRateSingleShot))
        (FiringMechanics|TrySpawnProjectile)))))

(fn FireBurst
  (Networking|SwitchHasAuthority
    (:Authority
      (Variables|CurrentState|SetCurrentShotInBurst (+ (Variables|CurrentState|GetCurrentShotInBurst) 1))
      (FiringMechanics|TrySpawnProjectile))))

(fn FireFullAuto
  (Networking|SwitchHasAuthority
    (:Authority
      (FiringMechanics|TrySpawnProjectile))))

(fn FireModeStep
  (switch Utilities|FlowControl|Switch|Switchon (Variables|CurrentState|GetCurrentFireMode)
    (:NewEnumerator0
      (Firemode|SetFireModeBurst))
    (:NewEnumerator1
      (Firemode|SetFireModeFullAuto))
    (:NewEnumerator2
      (Firemode|SetFireModeSingle))))

(fn SetFireModeSingle
  (if (Variables|Stats|GetSingleShot)
    (Firemode|SetFireMode)
    (else
      (Firemode|SetFireModeBurst))))

(fn SetFireMode
  (params (Firemode :type Byte :default 0))
  (Networking|SwitchHasAuthority
    (:Authority
      (switch Utilities|FlowControl|Switch|Switchon Firemode
        (:NewEnumerator0
          (if (Variables|Stats|GetSingleShot)
            (Variables|CurrentState|SetCurrentFireMode Firemode :!label _label)))
        (:NewEnumerator1
          (if (Variables|Stats|GetBurst)
            (goto _label)))
        (:NewEnumerator2
          (if (Variables|Stats|GetFullAuto)
            (goto _label)))))
    (:Remote
      (switch Utilities|FlowControl|Switch|Switchon Firemode
        (:NewEnumerator0
          (if (Variables|Stats|GetSingleShot)
            (Variables|CurrentState|SetCurrentFireMode Firemode :!label _label_2)))
        (:NewEnumerator1
          (if (Variables|Stats|GetBurst)
            (goto _label_2)))
        (:NewEnumerator2
          (if (Variables|Stats|GetFullAuto)
            (goto _label_2)))))))

(fn SetFireModeBurst
  (if (Variables|Stats|GetBurst)
    (Firemode|SetFireMode 0)
    (else
      (Firemode|SetFireModeFullAuto))))

(fn SetFireModeFullAuto
  (if (Variables|Stats|GetFullAuto)
    (Firemode|SetFireMode 0)
    (else
      (Firemode|SetFireModeBurst))))

(fn TrySpawnProjectile
  (bind _weaponmesh (Variables|Cosmetics|GetWeaponMesh))
  (bind _returnvalue (Transformation|GetSocketTransform _weaponmesh "Muzzle" "RTS_World"))
  (bind (_location _rotation) (Math|Transform|BreakTransform _returnvalue))
  (Networking|SwitchHasAuthority
    (:Authority
      (CallFunction|WillItJam)
      (if (Variables|CurrentState|GetIsJammed)
        ;[1 1 1] If you want to do something while jammed, do it here
        (Development|PrintString "Jammed!")
        (else
          (Variables|CurrentState|SetTimeSinceLastShot 0.0)
          (Variables|CurrentState|SetCurrentAmmo (- (Variables|CurrentState|GetCurrentAmmo) 1))
          ;[1 1 1] Setting all the variables of the projectile
          (Game|SpawnActorfromClass 0 (Math|Transform|MakeTransform _location _rotation) false 0)
          (Variables|Default|SetVelocity (* (Math|Vector|GetForwardVector _rotation) (Variables|Stats|GetMuzzleVelocity)))
          (Variables|Default|SetMass (Variables|Stats|GetBulletMass))
          (Variables|Stats|SetDrag (Variables|Stats|GetDrag))
          (Variables|Stats|SetCaliberDiameter (Variables|Stats|GetCaliberDiameter))
          (CallFunction|Initialize)
          (Audio|PlaySoundatLocation (Variables|Cosmetics|GetGunCue) _location)
          (Components|StaticMesh|SetStaticMesh (Variables|Cosmetics|GetProjectileMesh))
          (Variables|Stats|SetBaseDamage (Variables|Stats|GetBaseDamage)))))))

(fn HasAmmo
  (return (> (Variables|CurrentState|GetCurrentAmmo) 0)))

(fn TriggerNoAmmo
  (Development|PrintString "No ammo, CLICK!")
  (Variables|CurrentState|SetTriggerPulled false)
  ;[1 1 1] This is done to prevent burst completing after reload
  (Variables|CurrentState|SetCurrentShotInBurst 9000))

(fn SetIsJammed
  (params (IsJammed :type Boolean))
  (Networking|SwitchHasAuthority
    (:Authority
      (Variables|CurrentState|SetIsJammed IsJammed))))

(fn WillItJam
  (if (not (Variables|CurrentState|GetIsJammed))
    (Variables|CurrentState|SetIsJammed (> (Variables|Stats|GetJamRisk) (Math|Random|RandomFloatinRange 0.0 1e+02)))))

(fn SetIsTriggerPulled
  (params (TriggerPulled :type Boolean))
  (Variables|CurrentState|SetTriggerPulled TriggerPulled))