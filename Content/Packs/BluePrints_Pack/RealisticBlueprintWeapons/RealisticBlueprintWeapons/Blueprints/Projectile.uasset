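; Server-authoritative bullet projectile that simulates ballistics with gravity and velocity-squared drag derived from caliber, mass and air density.
; Each tick it line-traces along its next step, then either handles the impact or moves, orients to velocity and updates velocity.
; Impacts deal base damage scaled by remaining speed, then ricochet at shallow angles with reduced speed if allowed, otherwise destroy the actor.
; Initialize precomputes the drag factor, mass and initial speed.
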(event EventTick
  (params (DeltaSeconds :type Float%20%28single-precision%29))
  (Networking|SwitchHasAuthority
    (:Authority
      (Variables|Default|SetDeltaSeconds DeltaSeconds)
      (bind (_returnvalue _outhit) (CallFunction|Trace (Variables|Default|GetDeltaSeconds)))
      (if _returnvalue
        (CallFunction|Impact _outhit)
        (else
          (CallFunction|MoveProjectile (Variables|Default|GetDeltaSeconds))
          (CallFunction|ApplyGravity (Variables|Default|GetDeltaSeconds))
          (CallFunction|ApplyDrag (Variables|Default|GetDeltaSeconds)))))))

(fn ConstructionScript)

(fn ApplyGravity
  (params (DeltaSeconds :type Float%20%28single-precision%29))
  ;[1 1 1] Adds gravity component to the velocity. 9.8m per second.
  (Networking|SwitchHasAuthority
    (:Authority
      (Variables|Default|SetVelocity (+ (* "0, 0,-980.000000" DeltaSeconds) (Variables|Default|GetVelocity))))))

(fn ApplyDrag
  (params (DeltaSeconds :type Float%20%28single-precision%29))
  (Variables|Default|SetVelocity (* (Variables|Default|GetVelocity) (* (- (Math|Vector|VectorLength (Variables|Default|GetVelocity)) (* (* DeltaSeconds (* (Math|Float|Power (/ (Math|Vector|VectorLength (Variables|Default|GetVelocity)) 1e+02) 2.0) (/ (Variables|Default|GetD) (Variables|Default|GetMassInKg)))) 1e+02)) (/ 1.0 (Math|Vector|VectorLength (Variables|Default|GetVelocity)))))))

(fn Trace
  (params (DeltaSeconds :type Float%20%28single-precision%29))
  (bind _returnvalue (Transformation|GetActorLocation))
  ;[1 1 1] Here we're doing a line trace to see if we hit something
  (Networking|SwitchHasAuthority
    (:Authority
      (bind (_outhit _returnvalue_2) (Collision|LineTraceByChannel _returnvalue (+ (* (Variables|Default|GetVelocity) DeltaSeconds) _returnvalue) "TraceTypeQuery1" false 0 "Persistent" false))
      (return _returnvalue_2 _outhit))))

(fn MoveProjectile
  (params (DeltaSeconds :type Float%20%28single-precision%29))
  ;[1 1 1] Moving the projectile to its new location. Only server does this to prevent cheating
  (Networking|SwitchHasAuthority
    (:Authority
      (Transformation|SetActorLocation (+ (* (Variables|Default|GetVelocity) DeltaSeconds) (Transformation|GetActorLocation)) false)
      (Transformation|SetActorRotation (Math|Conversions|RotationFromXVector (Math|Vector|Normalize (Variables|Default|GetVelocity)))))))

(fn Impact
  (params (InHit :type Hit%20Result%20Structure))
  (bind (_bblockinghit _binitialoverlap _time _location _impactpoint _normal _impactnormal _physmat _hitactor) (Collision|BreakHitResult InHit))
  (Game|Damage|ApplyDamage _hitactor (* (/ (Math|Vector|VectorLength (Variables|Default|GetVelocity)) (Variables|Default|GetInitialSpeed)) (Variables|Default|GetBaseDamage)) 0 0)
  (if (and (Variables|Default|GetRicochet) (< (Class|KismetMathLibrary|DegAcos (Math|Vector|DotProduct _impactnormal (Math|Vector|Normalize (Variables|Default|GetVelocity)))) 122.0))
    ;[1 0.8142 -0.2389] Move to impact point(and slightly out to prevent getting caught inside mesh)
    (Transformation|SetActorLocation (+ _location (* _impactnormal 0.01)) false)
    ;[-0.1858 1 -0.8496] After ricochet we set velocity to 20% of impact speed
    (Variables|Default|SetVelocity (* (Math|Vector|MirrorVectorbyNormal (Variables|Default|GetVelocity) _impactnormal) 0.2))
    (else
      (Actor|DestroyActor))))

(fn Initialize
  (Variables|Default|SetD (/ (* (* (Variables|Default|GetAirDensity) (Variables|Default|GetDrag)) (Math|Float|MultiplybyPi (Math|Float|Power (/ (/ (Variables|Default|GetCaliberDiameter) 1e+03) 2.0) 2.0))) 2.0))
  (Variables|Default|SetMassInKg (/ (Variables|Default|GetMass) 1e+03))
  ;[1 1 1] We need the initial speed to calculate the damage
  (Variables|Default|SetInitialSpeed (Math|Vector|VectorLength (Variables|Default|GetVelocity))))