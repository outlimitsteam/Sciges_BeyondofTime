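; WeaponHUD is a HUD Blueprint that draws a weapon texture centered horizontally near the top of the screen.
; DrawHUD stores the screen dimensions each frame, then passes through a Gate that the Equip and Remove texture events open and close.
; While the gate is open, DrawWeaponTextures positions the texture relative to screen size and draws it at a fixed size.
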(event Custom|Remove_Texture_for_HUD
  (Utilities|FlowControl|Gate true) ; enters at Close
)

(event Custom|Equip_Texture_for_HUD
  (Utilities|FlowControl|Gate true) ; enters at Open
)

(event EventDrawHUD
  (params (SizeX :type Integer) (SizeY :type Integer))
  ;[1 1 1] This logic sets the variable 'Screen Dimensions' for use in further math
  (Variables|Default|SetScreen%20Dimensions (Math|Vector2D|MakeVector2D (Math|Conversions|ToFloat(Integer) SizeX) (Math|Conversions|ToFloat(Integer) SizeY)))
  (Utilities|FlowControl|Gate true ; This gate is used to control the drawing of the weapon textures
    (:Exit
      (CallFunction|DrawWeaponTextures) ; This function draws the weapon textures. Open for further info.
    )))

(fn ConstructionScript)

(fn DrawWeaponTextures
  (params (HUD%20Texture :type Texture%202D%20Object%20Reference))
  (bind _screen_dimensions (Variables|Default|GetScreen%20Dimensions))
  (bind (_x _y) (Math|Vector2D|BreakVector2D _screen_dimensions))
  (Canvas|DrawTexture HUD%20Texture (- (/ _x 2.0) 7e+01) (* (/ _y 2.0) 0.08) 1.4e+02 1e+02 0.0 0.0 1.0 1.0 "(R=1.000000,G=1.000000,B=1.000000,A=1.000000)") ; The values in this function define the width and height of the texture, no matter what its original dimensions are. This is also where the texture is plugged in to actually be drawn
)